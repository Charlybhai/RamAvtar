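; BP_Arrow1 is an arrow projectile that damages BP_Enemy_Base actors.
; Its Hit event ignores player character 0 and uses DoOnce so only the first other impact counts.
; An enemy hit applies fixed damage and plays a zombie sound at the arrow.
; Any counted impact disables Sphere collision and deactivates ProjectileMovement, then destroys the arrow after a short delay.
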(event EventBeginPlay)

(event Collision|EventActorBeginOverlap
  (params (OtherActor :type Actor%20Object%20Reference)))

(event EventTick
  (params (DeltaSeconds :type Float%20%28single-precision%29)))

(event Collision|EventHit
  (params (MyComp :type Primitive%20Component%20Object%20Reference) (Other :type Actor%20Object%20Reference) (OtherComp :type Primitive%20Component%20Object%20Reference) (bSelfMoved :type Boolean) (HitLocation :type Vector :default "0, 0, 0") (HitNormal :type Vector :default "0, 0, 0") (NormalImpulse :type Vector :default "0, 0, 0") (Hit :type Hit%20Result%20Structure%20%28by%20ref%29))
  (if (!= Other (Game|GetPlayerCharacter 0))
    (Utilities|FlowControl|DoOnce false
      (:Completed
        (Utilities|Casting|CastToBP_Enemy_Base Other
          (:then
            (Game|Damage|ApplyDamage Other 25.0 0 0)
            (Audio|PlaySoundatLocation "/Game/Free_Sounds_Pack/wav/Zombie_1_-_Short_1-01.Zombie_1_-_Short_1-01" (Transformation|GetActorLocation) "0, 0, 0" 1.0 1.0 0.0 0 0 0 0))
          (:CastFailed
            _))
        (Collision|SetCollisionEnabled (Variables|Default|GetSphere) "NoCollision")
        (Components|Activation|Deactivate (Variables|Default|GetProjectileMovement))
        (Utilities|FlowControl|Delay 3.0)
        (Actor|DestroyActor)))))

(fn ConstructionScript)