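; Base enemy Blueprint for a mutant that chases the player, attacks in melee and drops arrow and health pickups on death.
; It may roar at spawn when the player is distant, then loops AIMoveTo, a random attack with delayed damage (no range recheck) and idle.
; Self-calling events with Delays drive chasing and periodic roar sounds, playing animations directly on the mesh.
; Lethal damage unpossesses it, disables capsule collision and destroys it after timed delays.
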(event Custom|EnemyRoarLoop
  (Utilities|FlowControl|Delay (Math|Random|RandomFloatinRange 5.0 15.0))
  (if (> (Variables|Default|GetHealth) 0.0)
    (Audio|PlaySoundatLocation "/Game/Free_Sounds_Pack/wav/Creature_1-21.Creature_1-21" (Transformation|GetActorLocation) "0, 0, 0" 1.0 1.0 0.0 0 0 0 0)
    (CallFunction|EnemyRoarLoop)))

(event Custom|StartChase
  (if (not (Variables|Default|GetbIsDead))
    (Components|Animation|PlayAnimation (Variables|Character|GetMesh) "/Game/Enemies/Animations/mutant_run.mutant_run" true)
    (AI|AIMoveTo self "0, 0, 0" (Game|GetPlayerCharacter 0) 1.8e+02 false
      (:OnSuccess
        (bind _output_get (Variables|Default|SetCurrentAttack (.OutItem (Utilities|Array|Random (Variables|Default|GetAttackAnimations)))))
        (Components|Animation|PlayAnimation (Variables|Character|GetMesh) _output_get false)
        (Utilities|FlowControl|Delay 0.4)
        (Game|Damage|ApplyDamage (Game|GetPlayerCharacter 0) 2e+01 0 0)
        (Utilities|FlowControl|Delay (- (Animation|GetPlayLength _output_get) 0.4))
        (if (not (Variables|Default|GetbIsDead))
          (Components|Animation|PlayAnimation (Variables|Character|GetMesh) "/Game/Enemies/Animations/mutant_breathing_idle.mutant_breathing_idle" true)
          (Utilities|FlowControl|Delay 2.0)
          (CallFunction|StartChase)))
      (:OnFail
        (Utilities|FlowControl|Delay 0.2)
        (if (not (Variables|Default|GetbIsDead))
          (CallFunction|StartChase))))))

(event EventBeginPlay
  (if (and (> (Transformation|GetDistanceTo (Game|GetPlayerCharacter 0)) 1.2e+03) (not (Variables|Default|GetbHasRoared)))
    (Components|Animation|PlayAnimation (Variables|Character|GetMesh) (.OutItem (Utilities|Array|Random (Variables|Default|GetRoarAnimations))) false)
    (Utilities|FlowControl|Delay 4.0)
    (Variables|Default|SetbHasRoared true))
  (CallFunction|StartChase)
  (CallFunction|EnemyRoarLoop))

(event Collision|EventActorBeginOverlap
  (params (OtherActor :type Actor%20Object%20Reference)))

(event EventTick
  (params (DeltaSeconds :type Float%20%28single-precision%29)))

(event Game|Damage|EventAnyDamage
  (params (Damage :type Float%20%28single-precision%29) (DamageType :type Damage%20Type%20Object%20Reference) (InstigatedBy :type Controller%20Object%20Reference) (DamageCauser :type Actor%20Object%20Reference))
  (bind _returnvalue (Transformation|GetActorLocation))
  (if (not (Variables|Default|GetbIsDead))
    (bind _output_get (Variables|Default|SetHealth (- (Variables|Default|GetHealth) Damage)))
    (if (<= _output_get 0.0)
      (Variables|Default|SetbIsDead true)
      (Pawn|UnPossess (Pawn|GetController))
      (Components|Animation|PlayAnimation (Variables|Character|GetMesh) "/Game/Enemies/Animations/mutant_dying.mutant_dying" false)
      (Collision|SetCollisionEnabled (Variables|Collision|GetCapsuleComponent) "NoCollision")
      (Utilities|FlowControl|Delay 4.0)
      (Variables|/Script/Engine.SkeletalMeshComponent|SetbPauseAnims (Variables|Character|GetMesh) true)
      (Game|SpawnActorfromClass "/Game/BP_Arrow_Pickup.BP_Arrow_Pickup_C" (Math|Transform|MakeTransform _returnvalue "0, 0, 0" "1.000000,1.000000,1.000000") "Undefined" "MultiplyWithRoot" 0 0)
      (Game|SpawnActorfromClass "/Game/BP_Health_Pickup.BP_Health_Pickup_C" (Math|Transform|MakeTransform _returnvalue "0, 0, 0" "1.000000,1.000000,1.000000") "Undefined" "MultiplyWithRoot" 0 0)
      (Utilities|FlowControl|Delay 3.0)
      (Actor|DestroyActor))))

(fn ConstructionScript)