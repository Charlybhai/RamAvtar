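; BP_AgniBaan is a fire-arrow actor that decides the Ravan encounter by what it hits.
; Hitting BP_Ravan_Naabhi stops its glow, activates its RavanFire components, shows the victory UI and destroys the arrow.
; Any other hit except the player character, or a four-second timeout from BeginPlay, resets BP_WaveSpawner and destroys the arrow.
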(event Collision|EventHit
  (params (MyComp :type Primitive%20Component%20Object%20Reference) (Other :type Actor%20Object%20Reference) (OtherComp :type Primitive%20Component%20Object%20Reference) (bSelfMoved :type Boolean) (HitLocation :type Vector :default "0, 0, 0") (HitNormal :type Vector :default "0, 0, 0") (NormalImpulse :type Vector :default "0, 0, 0") (Hit :type Hit%20Result%20Structure%20%28by%20ref%29))
  (Utilities|Casting|CastToBP_ThirdPersonCharacter Other
    (:CastFailed
      (bind _asbp_ravan_naabhi (Utilities|Casting|CastToBP_Ravan_Naabhi Other)
        (:then
          (Default|StopGlowing _asbp_ravan_naabhi)
          (Components|Activation|Activate (Variables|/Game/BP_Ravan_Naabhi.BP_Ravan_Naabhi_C|GetRavanFire _asbp_ravan_naabhi) false)
          (Default|ShowVictoryUI _asbp_ravan_naabhi))
        (:CastFailed
          (bind _returnvalue (Actor|GetActorOfClass "/Game/BP_WaveSpawner.BP_WaveSpawner_C"))
          (Default|ResetSpawner _returnvalue)))
      (Actor|DestroyActor))))

(event EventBeginPlay
  (Utilities|FlowControl|Delay 4.0)
  (bind _returnvalue (Actor|GetActorOfClass "/Game/BP_WaveSpawner.BP_WaveSpawner_C"))
  (Default|ResetSpawner _returnvalue)
  (Actor|DestroyActor))

(fn ConstructionScript)