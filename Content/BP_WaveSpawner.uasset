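; BP_WaveSpawner runs four escalating enemy waves, then rewards the player with an AgniBaan pickup and makes the Ravan Naabhi glow.
; Each wave spawns as many enemies as the round number at random reachable points nearby, cycling three enemy classes from a random offset.
; OnDestroyed bindings count kills, starting the next wave after a short delay once all die.
; ResetSpawner stops the glow and restarts from round one.
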(event Custom|StartWave
  (Variables|Default|SetRandomOffset (Math|Random|RandomIntegerinRange 0 2))
  (for _index (range 1 (Variables|Default|GetCurrentRound))
    (Variables|Default|SetEnemiesAlive (+ (Variables|Default|GetEnemiesAlive) 1))
    (bind _returnvalue (Game|SpawnActorfromClass (Utilities|Select :Index (Math|Integer|%(Integer) (+ _index (Variables|Default|GetRandomOffset)) 3) :Option%200 "/Game/Enemies/BP_Enemy_Base.BP_Enemy_Base_C" :Option%201 "/Game/Enemies/BP_Enemy_02.BP_Enemy_02_C" :Option%202 "/Game/Enemies/BP_Enemy_03.BP_Enemy_03_C") (Math|Transform|MakeTransform (.RandomLocation (AI|Navigation|GetRandomReachablePointinRadius (Transformation|GetActorLocation) 1.5e+03 0 0))) "AlwaysSpawn" "MultiplyWithRoot" 0 0))
    (Game|BindEventtoOnDestroyed _returnvalue (delegate Custom|OnEnemyKilled))))

(event Custom|ResetSpawner
  (Variables|Default|SetCurrentRound 1)
  (Variables|Default|SetEnemiesAlive 0)
  (bind _returnvalue (Actor|GetActorOfClass "/Game/BP_Ravan_Naabhi.BP_Ravan_Naabhi_C"))
  (Default|StopGlowing _returnvalue)
  (CallFunction|StartWave))

(event Custom|OnEnemyKilled
  (params (DestroyedActor :type Actor%20Object%20Reference))
  (bind _output_get (Variables|Default|SetEnemiesAlive (- (Variables|Default|GetEnemiesAlive) 1)))
  (if (<= _output_get 0)
    (if (< (Variables|Default|GetCurrentRound) 4)
      (Variables|Default|SetCurrentRound (+ (Variables|Default|GetCurrentRound) 1))
      (Utilities|FlowControl|Delay 2.0)
      (CallFunction|StartWave)
      (else
        (Game|SpawnActorfromClass "/Game/BP_AgniBaan_Pickup.BP_AgniBaan_Pickup_C" (Math|Transform|MakeTransform (Transformation|GetActorLocation) "0, 0, 0" "1.000000,1.000000,1.000000") "AlwaysSpawn" "MultiplyWithRoot" 0 0)
        (bind _returnvalue (Actor|GetActorOfClass "/Game/BP_Ravan_Naabhi.BP_Ravan_Naabhi_C"))
        (Default|StartGlowing _returnvalue)))))

(event EventBeginPlay
  (CallFunction|StartWave))

(fn ConstructionScript)