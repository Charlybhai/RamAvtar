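; BP_Ravan_Naabhi is Ravan's navel actor, providing a toggleable glow and the victory sequence.
; StartGlowing and StopGlowing show and hide the NavelGlow component.
; ShowVictoryUI plays a fire sound at the actor, fires every BP_Firework in the level, then after a delay shows WBP_Victory with the mouse cursor and pauses the game.
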(event Custom|StopGlowing
  (Rendering|SetVisibility (Variables|Default|GetNavelGlow) false false))

(event Custom|StartGlowing
  (Rendering|SetVisibility (Variables|Default|GetNavelGlow) true false))

(event Custom|ShowVictoryUI
  (Audio|PlaySoundatLocation "/Game/Free_Sounds_Pack/wav/Fire_Burning_Loop_2.Fire_Burning_Loop_2" (Transformation|GetActorLocation) "0, 0, 0" 1.0 1.0 0.0 0 0 0 0)
  (bind _outactors (Actor|GetAllActorsOfClass "/Game/BP_Firework.BP_Firework_C"))
  (for _array_element _outactors
    (Default|FireRocket _array_element))
  (Utilities|FlowControl|Delay 1e+01)
  (bind _returnvalue (UserInterface|CreateWidget "/Game/WBP_Victory.WBP_Victory_C"))
  (UserInterface|Viewport|AddtoViewport _returnvalue 0)
  (Variables|/Script/Engine.PlayerController|SetbShowMouseCursor (Game|GetPlayerController 0) true)
  (Game|SetGamePaused true))

(fn ConstructionScript)