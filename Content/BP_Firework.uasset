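; Firework actor that launches a rocket trail upward and finishes with a sky burst when its FireRocket event is called.
; After a short random delay, it activates RocketTrail, plays the firework sound from an offset start time and moves the trail component upward over a few seconds.
; The trail then deactivates, and SkyBurst activates after a brief pause.
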(event Custom|FireRocket
  (Utilities|FlowControl|Delay (Math|Random|RandomFloatinRange 0.0 0.8))
  (Components|Activation|Activate (Variables|Default|GetRocketTrail) true)
  (Audio|PlaySoundatLocation "/Game/sfx/u_xg7ssi08yr-fireworks-379667.u_xg7ssi08yr-fireworks-379667" (Transformation|GetActorLocation) "0, 0, 0" 1.0 1.0 0.8 0 0 0 0)
  (Components|MoveComponentTo (Variables|Default|GetRocketTrail) "0.000000,0.000000,2000.000000" "0, 0, 0" false false 3.2 false)
  (Components|Activation|Deactivate (Variables|Default|GetRocketTrail))
  (Utilities|FlowControl|Delay 1.1)
  (Components|Activation|Activate (Variables|Default|GetSkyBurst) false))

(fn ConstructionScript)